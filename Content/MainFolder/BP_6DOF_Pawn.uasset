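; A six-degrees-of-freedom pawn that flies freely using player input.
; Look, turn and roll axes apply local rotations scaled by TurnSpeed, while Space and Ctrl nudge it along its local vertical axis.
; Every Tick, Shift selects maximum or minimum speed, and forward and right inputs move it along its own axes.
; Movement sets the transform directly without sweep collision or delta-time scaling, so it is frame-rate dependent.
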(event `self.ReceiveTick`
  (params (DeltaSeconds :type "Float (single-precision)"))
  (`|ExecutionSequence`
    (:`then_0`
      (if (`self.ShiftPressed`)
        (set `self.Speed` (`self.MaxSpeed`))
        (else
          (set `self.Speed` (`self.MinSpeed`)))))
    (:`then_1`
      (if (`self.SpacePressed`)
        (`self.K2_AddActorLocalOffset` (0.0 0.0 1.0))))
    (:`then_2`
      (if (`self.CtrlPressed`)
        (`self.K2_AddActorLocalOffset` (0.0 0.0 -1.0))))
    (:`then_3`
      (`self.K2_SetActorLocation` (+ (`self.K2_GetActorLocation`) (+ (* (`KismetMathLibrary.GetForwardVector` (`self.K2_GetActorRotation`)) (* (`self.GetInputAxisValue`) (`self.Speed`))) (* (`KismetMathLibrary.GetRightVector` (`self.K2_GetActorRotation`)) (* (`self.GetInputAxisValue`) (`self.Speed`)))))))))

(event `InputAxis|LookUp`
  (params (AxisValue :type "Float (single-precision)"))
  (`self.K2_AddActorLocalRotation` (`KismetMathLibrary.MakeRotator` 0.0 (* AxisValue (`self.TurnSpeed`)))))

(event `InputAction|Space`
  (params (Key :type "Key Structure"))
  (:`Pressed`
    (set `self.SpacePressed` true))
  (:`Released`
    (set `self.SpacePressed` false)))

(event `InputAxis|TurnAxis`
  (params (AxisValue :type "Float (single-precision)"))
  (`self.K2_AddActorLocalRotation` (`KismetMathLibrary.MakeRotator` 0.0 0.0 (* AxisValue (`self.TurnSpeed`)))))

(event `InputAction|Ctrl`
  (params (Key :type "Key Structure"))
  (:`Pressed`
    (set `self.CtrlPressed` true))
  (:`Released`
    (set `self.CtrlPressed` false)))

(event `InputAction|Shift`
  (params (Key :type "Key Structure"))
  (:`Pressed`
    (set `self.ShiftPressed` true))
  (:`Released`
    (set `self.ShiftPressed` false)))

(event `InputAxis|Roll`
  (params (AxisValue :type "Float (single-precision)"))
  (`self.K2_AddActorLocalRotation` (`KismetMathLibrary.MakeRotator` (* AxisValue (`self.TurnSpeed`)))))

(fn `UserConstructionScript`)